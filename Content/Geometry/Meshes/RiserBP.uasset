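; RiserBP is a level geometry actor that moves along a timeline after a delay and has a toggleable blocking capsule.
; On BeginPlay it stretches its Z scale by HeightMultiplier, waits DropOffset, then plays RiseLevel to teleport it from its start location by an offset scaled to that height.
; Every Tick it polls ThirdPersonGameMode's FlowOn, disabling BlockCapsule collision while true and enabling it otherwise.
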(event EventBeginPlay
  (Transformation|SetActorScale3D (* (Transformation|GetActorScale3D) (Math|Vector|MakeVector 1.0 1.0 (Variables|Default|GetheightMultiplier))))
  (bind _output_get (Variables|Default|SetInitialPos (Transformation|GetActorLocation)))
  (Utilities|FlowControl|Delay (Variables|Default|GetdropOffset))
  (bind _level (Timeline|RiseLevel PlayFromStart)
    (:Update
      (Transformation|SetActorLocation (+ (* _level (* 180 (Variables|Default|GetheightMultiplier))) _output_get) false true))))

(event EventTick
  (params (DeltaSeconds :type Float%20%28single-precision%29))
  (bind _blockcapsule (Variables|Default|GetBlockCapsule))
  (bind _asthird_person_game_mode (Utilities|Casting|CastToThirdPersonGameMode (Game|GetGameMode)))
  (if (Variables|/Game/ThirdPersonBP/Blueprints/ThirdPersonGameMode.ThirdPersonGameMode_C|GetflowOn _asthird_person_game_mode)
    (Collision|SetCollisionEnabled _blockcapsule "NoCollision")
    (else
      (Collision|SetCollisionEnabled _blockcapsule "QueryAndPhysics"))))

(fn ConstructionScript)